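; BP_GridTile is one clickable tile of a grid, showing ground type, selection and path state.
; It forwards cursor and click events to BpGrid and reads its tile data there by GridIndex.
; SetTileColor drives material parameters from those states, while debug events tint tiles for pathfinding open and closed sets.
; On BeginPlay, after a short delay, it colors itself, scales to the grid's tile size and initializes its widget.
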(event OnBeginCursorOver(StaticMesh)
  (params (TouchedComponent :type Primitive%20Component%20Object%20Reference))
  (CallFunction|EventStartOverTile)
  (Default|EventNewTileOvered (Variables|Grid|Getbp_Grid) self))

(event OnEndCursorOver(StaticMesh)
  (params (TouchedComponent :type Primitive%20Component%20Object%20Reference))
  (Default|EventNewTileOvered (Variables|Grid|Getbp_Grid) self))

(event OnClicked(StaticMesh)
  (params (TouchedComponent :type Primitive%20Component%20Object%20Reference) (ButtonPressed :type Key%20Structure :default "None"))
  (CallFunction|EventSelectTile)
  (Default|EventNewTileSelected (Variables|Grid|Getbp_Grid) self))

(event Custom|Event_SelectTile
  (Variables|Grid|SetbIsSelected true)
  (Development|PrintString "Tile Selected")
  (Grid|SetTileColor))

(event Custom|Event_DeselectTile
  (Variables|Grid|SetbIsSelected false)
  (Development|PrintString "Tile Deselcted")
  (Grid|SetTileColor))

(event Custom|Event_StartOverTile
  (Variables|Grid|SetbIsSelected true)
  (Grid|SetTileColor))

(event Custom|Event_EndOverTile
  (Variables|Grid|SetbIsSelected false)
  (Grid|SetTileColor))

(event Custom|Event_IsInPath
  (params (isInPath :type Boolean))
  (Variables|Default|SetbIsInPath isInPath)
  (Grid|SetTileColor))

(event Custom|DebugEvent_OpenSet
  (Rendering|Material|SetVectorParameterValueonMaterials (Variables|Default|GetStaticMesh) "TileColor" (Math|Conversions|ToVector(LinearColor) "(R=0.808409,G=0.102694,B=0.859375,A=1.000000)")))

(event Custom|DebugEvent_ClosedSet
  (Rendering|Material|SetVectorParameterValueonMaterials (Variables|Default|GetStaticMesh) "TileColor" (Math|Conversions|ToVector(LinearColor) "(R=0.331252,G=1.000000,B=0.233968,A=1.000000)")))

(event EventBeginPlay
  (Utilities|FlowControl|Delay 0.2)
  (Grid|SetTileColor)
  (Grid|SetTileSize)
  (Debug|SetWidgetVariables))

(fn ConstructionScript)

(fn SetTileColor
  (Utilities|FlowControl|Sequence
    (:then_0
      (switch Utilities|FlowControl|Switch|SwitchonEnum_GroundTypes (.groundtype (Grid|GetTileData))
        (:NewEnumerator0
          (LocalVariables|SetTileColor "(R=0.000000,G=0.947917,B=0.897680,A=1.000000)"))
        (:NewEnumerator1
          (LocalVariables|SetTileColor "(R=1.000000,G=0.919217,B=0.224955,A=1.000000)"))
        (:NewEnumerator2
          (LocalVariables|SetTileColor "(R=0.994792,G=0.160878,B=0.101458,A=1.000000)"))
        (:NewEnumerator3
          (LocalVariables|SetTileColor "(R=1.000000,G=0.000000,B=0.067033,A=1.000000)"))
        (:NewEnumerator4
          (LocalVariables|SetTileColor "(R=1.000000,G=0.962442,B=0.997690,A=1.000000)"))))
    (:then_1
      (if (Variables|Grid|GetbIsSelected)
        (Rendering|Material|SetScalarParameterValueonMaterials (Variables|Default|GetStaticMesh) "bIsSelected" 1.0)
        (else
          (Rendering|Material|SetScalarParameterValueonMaterials (Variables|Default|GetStaticMesh) "bIsSelected" 0.0))))
    (:then_2
      (if (Variables|Grid|GetbIsOvered)
        (LocalVariables|SettileColor (Math|Conversions|ToLinearColor(Vector) (* (Math|Conversions|ToVector(LinearColor) (LocalVariables|GettileColor)) 3.0)))))
    (:then_3
      (if (Variables|Default|GetbIsInPath)
        (LocalVariables|SetTileColor "(R=0.603664,G=0.187433,B=1.000000,A=1.000000)")))
    (:then_4
      (Rendering|Material|SetVectorParameterValueonMaterials (Variables|Default|GetStaticMesh) "TileColor" (Math|Conversions|ToVector(LinearColor) (LocalVariables|GettileColor))))))

(fn GetTileData
  (return (.Value (Utilities|Map|Find (Variables|/Game/Blueprints/Grid/BP_Grid.BP_Grid_C|Getstruct_Tiles (Variables|Grid|Getbp_Grid)) (Variables|Grid|GetgridIndex\)))))

(fn SetTileSize
  (bind _bp_grid (Variables|Grid|Getbp_Grid))
  (bind _staticmesh (Variables|Default|GetStaticMesh))
  (bind _returnvalue (Transformation|GetWorldScale _staticmesh))
  (bind _tilesize (Variables|/Game/Blueprints/Grid/BP_Grid.BP_Grid_C|GetTileSize _bp_grid))
  (bind _returnvalue_2 (/ _tilesize 5e+01))
  (bind _returnvalue_3 (* _returnvalue _returnvalue_2))
  (Transformation|SetWorldScale3D _staticmesh (Math|Vector|MakeVector (.x _returnvalue_3) (.y _returnvalue_3) 1.0)))

(fn SetWidgetVariables
  (bind _widget (Variables|Default|GetWidget))
  (bind _returnvalue (UserInterface|GetUserWidgetObject _widget))
  (bind _asw_grid_tile (Utilities|Casting|CastToW_GridTile _returnvalue))
  (Variables|/Game/Blueprints/Grid/W_GridTile.W_GridTile_C|Setgrid _asw_grid_tile (Variables|Grid|Getbp_Grid))
  (Variables|/Game/Blueprints/Grid/W_GridTile.W_GridTile_C|SetgridIndex\ _asw_grid_tile (Variables|Grid|GetgridIndex\)))