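; BP_PlayerController is a player controller that provides two keyboard toggles, apparently for debugging or inspection.
; R alternates through a FlipFlop between hiding and showing every BP_Base_Obstacle actor in the level, gathered with GetAllActorsOfClass on each press.
; T alternates global time dilation between slow motion and normal speed.
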(event Input|KeyboardEvents|R
  (params (Key :type Key%20Structure :default "None"))
  (:Pressed
    (Utilities|FlowControl|FlipFlop
      (:A
        (bind _outactors (Actor|GetAllActorsOfClass "/Game/Blueprints/Grid/BP_Base_Obstacle.BP_Base_Obstacle_C"))
        (for _array_element _outactors
          (Rendering|SetActorHiddenInGame _array_element true)))
      (:B
        (bind _outactors_2 (Actor|GetAllActorsOfClass "/Game/Blueprints/Grid/BP_Base_Obstacle.BP_Base_Obstacle_C"))
        (for _array_element_2 _outactors_2
          (Rendering|SetActorHiddenInGame _array_element_2 false))))))

(event Input|KeyboardEvents|T
  (params (Key :type Key%20Structure :default "None"))
  (:Pressed
    (Utilities|FlowControl|FlipFlop
      (:A
        (Utilities|Time|SetGlobalTimeDilation 0.1))
      (:B
        (Utilities|Time|SetGlobalTimeDilation 1.0)))))

(fn ConstructionScript)